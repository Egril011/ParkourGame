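; BP_Timer is a countdown Blueprint that shows the lose screen when the player's time runs out.
; On BeginPlay it starts a looping timer that subtracts TimeInter from PlayerTimeRemaining in BP_MyGameInstance on each tick.
; When the reduced time minus another interval would fall below zero, it clears the timer and adds a WBP_lose widget to the viewport.
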(event EventBeginPlay
  (Utilities|Time|SetTimerbyFunctionName 0 "Timer" (Variables|Default|GetTimeInter) true))

(fn ConstructionScript)

(fn Timer
  (bind _asbp_my_game_instance (Utilities|Casting|CastToBP_MyGameInstance (Game|GetGameInstance)))
  (Variables|/Game/Blueprint/GameInstace/BP_MyGameInstance.BP_MyGameInstance_C|SetPlayerTimeRemaining _asbp_my_game_instance (- (Variables|/Game/Blueprint/GameInstace/BP_MyGameInstance.BP_MyGameInstance_C|GetPlayerTimeRemaining _asbp_my_game_instance) (Variables|Default|GetTimeInter)))
  (if (< (- (Variables|/Game/Blueprint/GameInstace/BP_MyGameInstance.BP_MyGameInstance_C|GetPlayerTimeRemaining _asbp_my_game_instance) (Variables|Default|GetTimeInter)) 0.0)
    (Utilities|Time|ClearTimerbyFunctionName 0 "Timer")
    (bind _returnvalue (UserInterface|CreateWidget "/Game/UI/WBP_lose.WBP_lose_C"))
    (UserInterface|Viewport|AddtoViewport _returnvalue 0)
    (else
      (return))))