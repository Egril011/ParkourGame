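; Double jump pickup item that tints its mesh purple, adds itself to the game instance's inventory on Interact, then destroys itself.
; Usable sets IsDoubleJumpOn and adds a countdown widget to the item effect UI.
; A looping timer updates the countdown, raising the player's JumpMaxCount to 2 once.
; On expiry it restores one jump, removes the widget and clears the timer, but sets IsDoubleJumpOn true again rather than false.
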(event EventBeginPlay
  (|CallParentFunction)
  (Rendering|Material|SetVectorParameterValueonMaterials (Variables|Default|GetStaticMesh) "Colour" (Math|Conversions|ToVector(LinearColor) "(R=0.615686,G=0.000000,B=1.000000,A=1.000000)")))

(event Collision|EventActorBeginOverlap
  (params (OtherActor :type Actor%20Object%20Reference))
  (|CallParentFunction OtherActor) ; This node is disabled and will not be called.\nDrag off pins to build functionality.
)

(event EventTick
  (params (DeltaSeconds :type Float%20%28single-precision%29))
  (|CallParentFunction DeltaSeconds) ; This node is disabled and will not be called.\nDrag off pins to build functionality.
)

(event EventInteract
  (bind _asbp_first_person_game_mode (Utilities|Casting|CastToBP_FirstPersonGameMode (Game|GetGameMode)))
  (bind _asbp_my_game_instance (Utilities|Casting|CastToBP_MyGameInstance (Game|GetGameInstance)))
  (bind _tempinventory1 (Default|AddItem (Variables|/Game/FirstPerson/Blueprints/BP_FirstPersonGameMode.BP_FirstPersonGameMode_C|GetInventory _asbp_first_person_game_mode) "Doube Jump" 1 (Utilities|GetClass self) (Variables|/Game/Blueprint/GameInstace/BP_MyGameInstance.BP_MyGameInstance_C|GetPlayerInventory _asbp_my_game_instance)))
  (Variables|/Game/Blueprint/GameInstace/BP_MyGameInstance.BP_MyGameInstance_C|SetPlayerInventory _asbp_my_game_instance _tempinventory1)
  (Actor|DestroyActor))

(event EventUsable
  (bind _asbp_my_game_instance (Utilities|Casting|CastToBP_MyGameInstance (Game|GetGameInstance)))
  (Variables|/Game/Blueprint/GameInstace/BP_MyGameInstance.BP_MyGameInstance_C|SetIsDoubleJumpOn _asbp_my_game_instance true)
  (bind _asbp_first_person_game_mode (Utilities|Casting|CastToBP_FirstPersonGameMode (Game|GetGameMode)))
  (bind _returnvalue (UserInterface|CreateWidget "/Game/UI/Items/WBP_ItemEffectSlot.WBP_ItemEffectSlot_C"))
  (bind _output_get (Variables|Default|SetWidgetRef _returnvalue))
  (Variables|/Script/UMG.TextBlock|SetText (Variables|/Game/UI/Items/WBP_ItemEffectSlot.WBP_ItemEffectSlot_C|GetTextBlock_0 _output_get) (Utilities|Text|ToText(String) (Utilities|String|Append "Double Jump: " (Utilities|String|ToString(Float) (Variables|Default|GetTimer)))))
  (Class|VerticalBox|AddChildtoVerticalBox (Variables|/Game/UI/Items/WBP_ItemEffect.WBP_ItemEffect_C|GetVerticalBoxItemEffect (Variables|/Game/FirstPerson/Blueprints/BP_FirstPersonGameMode.BP_FirstPersonGameMode_C|GetItemEffectWidget _asbp_first_person_game_mode)) (Variables|/Game/UI/Items/WBP_ItemEffectSlot.WBP_ItemEffectSlot_C|GetVerticalBoxItemEffectSlot _returnvalue))
  (Layout|BorderSlot|SetPadding (Variables|/Game/FirstPerson/Blueprints/BP_FirstPersonGameMode.BP_FirstPersonGameMode_C|GetItemEffectWidget _asbp_first_person_game_mode) (Utilities|Struct|MakeMargin 0.0 0.0 0.0 3e+01) :!class /Script/UMG.UserWidget)
  (Utilities|Time|SetTimerbyFunctionName 0 "DoubleJump" (Variables|Default|GetTime) true))

(fn ConstructionScript
  (|CallParentFunction))

(fn DoubleJump
  (bind _output_get (Variables|Default|SetTimer (- (Variables|Default|GetTimer) (Variables|Default|GetTime))))
  (Variables|/Script/UMG.TextBlock|SetText (Variables|/Game/UI/Items/WBP_ItemEffectSlot.WBP_ItemEffectSlot_C|GetTextBlock_0 (Variables|Default|GetWidgetRef)) (Utilities|Text|ToText(String) (Utilities|String|Append "Double Jump: " (Utilities|String|ToString(Float) (Variables|Default|GetTimer)))))
  (if (> _output_get 0.0)
    (if (Variables|Default|GetFirstExecution)
      (return)
      (else
        (bind _asbp_first_person_character (Utilities|Casting|CastToBP_FirstPersonCharacter (Game|GetPlayerCharacter 0)))
        (Variables|/Script/Engine.Character|SetJumpMaxCount _asbp_first_person_character 2)
        (Variables|Default|SetFirstExecution true)
        (return)))
    (else
      (bind _asbp_first_person_character_2 (Utilities|Casting|CastToBP_FirstPersonCharacter (Game|GetPlayerCharacter 0)))
      (Variables|/Script/Engine.Character|SetJumpMaxCount _asbp_first_person_character_2 1)
      (Widget|RemovefromParent (Variables|/Game/UI/Items/WBP_ItemEffectSlot.WBP_ItemEffectSlot_C|GetVerticalBoxItemEffectSlot (Variables|Default|GetWidgetRef)))
      (Variables|Default|SetFirstExecution false)
      (bind _asbp_my_game_instance (Utilities|Casting|CastToBP_MyGameInstance (Game|GetGameInstance)))
      (Variables|/Game/Blueprint/GameInstace/BP_MyGameInstance.BP_MyGameInstance_C|SetIsDoubleJumpOn _asbp_my_game_instance true)
      (Utilities|Time|ClearTimerbyFunctionName 0 "DoubleJump"))))