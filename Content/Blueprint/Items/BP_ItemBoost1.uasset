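; BP_ItemBoost1 is a "Speed boost" pickup item that goes into the player's inventory.
; Interact adds it through the game mode's Inventory, stores the result in the game instance's PlayerInventory, briefly shows a W_Text inventory hint, then destroys the actor.
; Usable looks the item up in that inventory but does nothing with the result, so no boost effect is implemented here.
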(event EventBeginPlay
  (|CallParentFunction) ; This node is disabled and will not be called.\nDrag off pins to build functionality.
)

(event Collision|EventActorBeginOverlap
  (params (OtherActor :type Actor%20Object%20Reference))
  (|CallParentFunction OtherActor) ; This node is disabled and will not be called.\nDrag off pins to build functionality.
)

(event EventTick
  (params (DeltaSeconds :type Float%20%28single-precision%29))
  (|CallParentFunction DeltaSeconds) ; This node is disabled and will not be called.\nDrag off pins to build functionality.
)

(event EventInteract
  (bind _asbp_first_person_game_mode (Utilities|Casting|CastToBP_FirstPersonGameMode (Game|GetGameMode)))
  (bind _asbp_my_game_instance (Utilities|Casting|CastToBP_MyGameInstance (Game|GetGameInstance)))
  (bind _tempinventory1 (Default|AddItem (Variables|/Game/FirstPerson/Blueprints/BP_FirstPersonGameMode.BP_FirstPersonGameMode_C|GetInventory _asbp_first_person_game_mode) "Speed boost" 1 (Utilities|GetClass self) (Variables|/Game/Blueprint/GameInstace/BP_MyGameInstance.BP_MyGameInstance_C|GetPlayerInventory _asbp_my_game_instance)))
  (Variables|/Game/Blueprint/GameInstace/BP_MyGameInstance.BP_MyGameInstance_C|SetPlayerInventory _asbp_my_game_instance _tempinventory1)
  (bind _returnvalue (UserInterface|CreateWidget "/Game/UI/W_Text.W_Text_C"))
  (Variables|/Script/UMG.TextBlock|SetText (Variables|/Game/UI/W_Text.W_Text_C|GetTextBlock_0 _returnvalue) "You can press 'Tab' to see your inventory and use your items.")
  (UserInterface|Viewport|AddtoViewport _returnvalue 0)
  (Utilities|FlowControl|Delay 0.5)
  (Widget|RemovefromParent _returnvalue)
  (Actor|DestroyActor))

(event EventUsable
  (bind _asbp_first_person_game_mode (Utilities|Casting|CastToBP_FirstPersonGameMode (Game|GetGameMode)))
  (bind _asbp_my_game_instance (Utilities|Casting|CastToBP_MyGameInstance (Game|GetGameInstance)))
  (if (.Is%20Found (Default|FindItem (Variables|/Game/FirstPerson/Blueprints/BP_FirstPersonGameMode.BP_FirstPersonGameMode_C|GetInventory _asbp_first_person_game_mode) "Speed boost" (Variables|/Game/Blueprint/GameInstace/BP_MyGameInstance.BP_MyGameInstance_C|GetPlayerInventory _asbp_my_game_instance)))
    _))

(fn ConstructionScript
  (|CallParentFunction))