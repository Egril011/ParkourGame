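; BP_PowerCellTutoriel is an interactable Power Cell pickup, apparently for the tutorial, that plays an audio component from BeginPlay.
; On Interact it stops the audio and calls AddItem on the first-person game mode's Inventory, passing one Power Cell and its own class.
; The returned inventory is written back to PlayerInventory on the game instance, then the actor destroys itself.
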(event EventBeginPlay
  (|CallParentFunction)
  (Audio|Components|Audio|Play (Variables|Default|GetAudio) 0.0))

(event Collision|EventActorBeginOverlap
  (params (OtherActor :type Actor%20Object%20Reference))
  (|CallParentFunction OtherActor) ; This node is disabled and will not be called.\nDrag off pins to build functionality.
)

(event EventTick
  (params (DeltaSeconds :type Float%20%28single-precision%29))
  (|CallParentFunction DeltaSeconds) ; This node is disabled and will not be called.\nDrag off pins to build functionality.
)

(event EventInteract
  (Audio|Components|Audio|Stop (Variables|Default|GetAudio))
  (bind _asbp_first_person_game_mode (Utilities|Casting|CastToBP_FirstPersonGameMode (Game|GetGameMode)))
  (bind _asbp_my_game_instance (Utilities|Casting|CastToBP_MyGameInstance (Game|GetGameInstance)))
  (bind _tempinventory1 (Default|AddItem (Variables|/Game/FirstPerson/Blueprints/BP_FirstPersonGameMode.BP_FirstPersonGameMode_C|GetInventory _asbp_first_person_game_mode) "Power Cell" 1 (Utilities|GetClass self) (Variables|/Game/Blueprint/GameInstace/BP_MyGameInstance.BP_MyGameInstance_C|GetPlayerInventory _asbp_my_game_instance)))
  (Variables|/Game/Blueprint/GameInstace/BP_MyGameInstance.BP_MyGameInstance_C|SetPlayerInventory _asbp_my_game_instance _tempinventory1)
  (Actor|DestroyActor))

(fn ConstructionScript
  (|CallParentFunction))