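; Inventory manager that registers itself on BP_FirstPersonGameMode at begin play if none is set, providing item add, find and use logic.
; It operates on item-struct arrays passed in by callers, with AddItem stacking quantities by name or appending new entries.
; UseItem handles BPI_Usable classes by decrementing quantity, without a zero check or removal, then spawning a hidden actor at the origin to receive UsableMessage.
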(event EventBeginPlay
  (bind _asbp_first_person_game_mode (Utilities|Casting|CastToBP_FirstPersonGameMode (Game|GetGameMode)))
  (Utilities|IsValid (Variables|/Game/FirstPerson/Blueprints/BP_FirstPersonGameMode.BP_FirstPersonGameMode_C|GetInventory _asbp_first_person_game_mode)
    (:Is%20Not%20Valid
      (Variables|/Game/FirstPerson/Blueprints/BP_FirstPersonGameMode.BP_FirstPersonGameMode_C|SetInventory _asbp_first_person_game_mode self))))

(fn ConstructionScript)

(fn FindItem
  (params (ItemName :type String) (Inventory :type Array%20of%20BPS%20Item%20Structs%20Structures))
  (for (_array_element _array_index) Inventory
    (if (Utilities|Enum|Equal(Enum) (.ItemName (Utilities|Struct|BreakBPS_ItemStructs _array_element)) ItemName)
      (LocalVariables|SetItemIsFound true)
      (LocalVariables|SetItemIndex _array_index)))
  (return (LocalVariables|GetItemIsFound) (LocalVariables|GetItemIndex)))

(fn AddItem
  (params (ItemName :type String) (ItemQuantity :type Integer) (ClassReference :type Actor%20Class%20Reference) (Inventory :type Array%20of%20BPS%20Item%20Structs%20Structures))
  (LocalVariables|SetTempName ItemName)
  (LocalVariables|SetTempQuantity ItemQuantity)
  (LocalVariables|SetActor%20Reference ClassReference)
  (bind _output_get (LocalVariables|SetTemp%20Inventory Inventory))
  (if (> (Utilities|Array|Length _output_get) 0)
    (if (.Is%20Found (CallFunction|FindItem (LocalVariables|GetTempName) (LocalVariables|GetTemp%20Inventory)))
      (Utilities|Array|SetArrayElem (LocalVariables|GetTemp%20Inventory) (.Index (CallFunction|FindItem (LocalVariables|GetTempName) (LocalVariables|GetTemp%20Inventory))) (Utilities|Struct|MakeBPS_ItemStructs (.ItemName (Utilities|Struct|BreakBPS_ItemStructs (Utilities|Array|Get(acopy) (LocalVariables|GetTemp%20Inventory) (.Index (CallFunction|FindItem (LocalVariables|GetTempName) (LocalVariables|GetTemp%20Inventory)))))) (+ (.ItemQuantity (Utilities|Struct|BreakBPS_ItemStructs (Utilities|Array|Get(acopy) (LocalVariables|GetTemp%20Inventory) (.Index (CallFunction|FindItem (LocalVariables|GetTempName) (LocalVariables|GetTemp%20Inventory)))))) (LocalVariables|GetTempQuantity)) (.ItemActorClass (Utilities|Struct|BreakBPS_ItemStructs (Utilities|Array|Get(acopy) (LocalVariables|GetTemp%20Inventory) (.Index (CallFunction|FindItem (LocalVariables|GetTempName) (LocalVariables|GetTemp%20Inventory))))))))
      (return (LocalVariables|GetTemp%20Inventory))
      (else
        (Utilities|Array|Add (LocalVariables|GetTemp%20Inventory) (Utilities|Struct|MakeBPS_ItemStructs (LocalVariables|GetTempName) (LocalVariables|GetTempQuantity) (LocalVariables|GetActor%20Reference)))
        (return (LocalVariables|GetTemp%20Inventory))))
    (else
      (Utilities|Array|Add (LocalVariables|GetTemp%20Inventory) (Utilities|Struct|MakeBPS_ItemStructs (LocalVariables|GetTempName) (LocalVariables|GetTempQuantity) (LocalVariables|GetActor%20Reference)))
      (return (LocalVariables|GetTemp%20Inventory)))))

(fn UseItem
  (params (Inventory :type Array%20of%20BPS%20Item%20Structs%20Structures) (ItemName :type String))
  (bind (_is_found _index) (CallFunction|FindItem ItemName Inventory))
  (if _is_found
    (bind _output_get (LocalVariables|SetIndex _index))
    (if (Class|KismetSystemLibrary|DoesClassImplementInterface (.ItemActorClass (Utilities|Struct|BreakBPS_ItemStructs (Utilities|Array|Get(acopy) Inventory _output_get))) "/Game/Blueprint/ItemsInteraction/BPI_Usable.BPI_Usable_C")
      (bind _result (Math|Integer|DecrementInt (.ItemQuantity (Utilities|Struct|BreakBPS_ItemStructs (Utilities|Array|Get(acopy) Inventory _output_get))))
        (:%20%20
          (Utilities|Array|SetArrayElem Inventory (LocalVariables|GetIndex) (Utilities|Struct|MakeBPS_ItemStructs (.ItemName (Utilities|Struct|BreakBPS_ItemStructs (Utilities|Array|Get(acopy) Inventory _output_get))) _result (.ItemActorClass (Utilities|Struct|BreakBPS_ItemStructs (Utilities|Array|Get(acopy) Inventory _output_get)))))
          (bind _returnvalue (Game|SpawnActorfromClass (.ItemActorClass (Utilities|Struct|BreakBPS_ItemStructs (Utilities|Array|Get(acopy) Inventory _output_get))) (Math|Transform|MakeTransform "0, 0, 0") "Undefined" "MultiplyWithRoot" 0 0))
          (Rendering|SetActorHiddenInGame _returnvalue true)
          (Class|BPIUsable|Usable(Message) _returnvalue)
          (return)))
      (else
        (return)))
    (else
      (return))))