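; BP_PlayerRespawn is a checkpoint actor that records where the first-person player respawns.
; When the player character's capsule overlaps its Box, it compares the SceneRespawn component's world location to the respawn transform saved in BP_MyGameInstance.
; If they differ, it stores SceneRespawn's location and rotation there with unit scale and prints the new location.
; The respawn itself is not performed in this Blueprint.
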(event OnComponentBeginOverlap(Box)
  (params (OverlappedComponent :type Primitive%20Component%20Object%20Reference) (OtherActor :type Actor%20Object%20Reference) (OtherComp :type Primitive%20Component%20Object%20Reference) (OtherBodyIndex :type Integer) (bFromSweep :type Boolean) (SweepResult :type Hit%20Result%20Structure%20%28by%20ref%29))
  (bind _scenerespawn (Variables|Default|GetSceneRespawn))
  (bind _asbp_first_person_character (Utilities|Casting|CastToBP_FirstPersonCharacter OtherActor))
  (if (== (Variables|/Script/Engine.Character|GetCapsuleComponent _asbp_first_person_character) OtherComp)
    (bind _asbp_my_game_instance (Utilities|Casting|CastToBP_MyGameInstance (Game|GetGameInstance)))
    (Variables|Default|SetCheckPointLocation (Transformation|GetWorldLocation (Variables|Default|GetSceneRespawn)))
    (if (not (Utilities|Operators|EqualEqual (.location (Variables|/Game/Blueprint/GameInstace/BP_MyGameInstance.BP_MyGameInstance_C|GetPlayerRespawn _asbp_my_game_instance)) (Variables|Default|GetCheckPointLocation) 0.0))
      (bind _output_get (Variables|/Game/Blueprint/GameInstace/BP_MyGameInstance.BP_MyGameInstance_C|SetPlayerRespawn _asbp_my_game_instance (Math|Transform|MakeTransform (Transformation|GetWorldLocation _scenerespawn) (Transformation|GetWorldRotation _scenerespawn) "1.000000,1.000000,1.000000")))
      (Development|PrintString (Utilities|String|ToString(Vector) (.location _output_get))))))

(event EventBeginPlay)

(fn ConstructionScript)