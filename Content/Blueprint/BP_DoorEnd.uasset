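; BP_DoorEnd is an end-door actor whose interaction triggers the win screen when the player holds Power Cells.
; On Interact it searches the GameInstance's inventory through the GameMode's Inventory, requiring a quantity of exactly four.
; Success removes that entry and shows WBP_Win, passing it a linked list.
; Failure shows a timed W_Text hint, whose stored reference blocks further interaction until it disappears.
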(event EventBeginPlay
  (|CallParentFunction) ; This node is disabled and will not be called.\nDrag off pins to build functionality.
)

(event Collision|EventActorBeginOverlap
  (params (OtherActor :type Actor%20Object%20Reference))
  (|CallParentFunction OtherActor) ; This node is disabled and will not be called.\nDrag off pins to build functionality.
)

(event EventTick
  (params (DeltaSeconds :type Float%20%28single-precision%29))
  (|CallParentFunction DeltaSeconds) ; This node is disabled and will not be called.\nDrag off pins to build functionality.
)

(event EventInteract
  (Utilities|IsValid (Variables|Default|GetWidgetReference)
    (:Is%20Not%20Valid
      (bind _asbp_my_game_instance (Utilities|Casting|CastToBP_MyGameInstance (Game|GetGameInstance)))
      (bind _asbp_first_person_game_mode (Utilities|Casting|CastToBP_FirstPersonGameMode (Game|GetGameMode)))
      (if (.Is%20Found (Default|FindItem (Variables|/Game/FirstPerson/Blueprints/BP_FirstPersonGameMode.BP_FirstPersonGameMode_C|GetInventory _asbp_first_person_game_mode) "Power Cell" (Variables|/Game/Blueprint/GameInstace/BP_MyGameInstance.BP_MyGameInstance_C|GetPlayerInventory _asbp_my_game_instance)))
        (if (== (.ItemQuantity (Utilities|Struct|BreakBPS_ItemStructs (Utilities|Array|Get(acopy) (Variables|/Game/Blueprint/GameInstace/BP_MyGameInstance.BP_MyGameInstance_C|GetPlayerInventory _asbp_my_game_instance) (.Index (Default|FindItem (Variables|/Game/FirstPerson/Blueprints/BP_FirstPersonGameMode.BP_FirstPersonGameMode_C|GetInventory _asbp_first_person_game_mode) "Power Cell" (Variables|/Game/Blueprint/GameInstace/BP_MyGameInstance.BP_MyGameInstance_C|GetPlayerInventory _asbp_my_game_instance)))))) 4)
          (Utilities|Array|RemoveIndex (Variables|/Game/Blueprint/GameInstace/BP_MyGameInstance.BP_MyGameInstance_C|GetPlayerInventory _asbp_my_game_instance) (.Index (Default|FindItem (Variables|/Game/FirstPerson/Blueprints/BP_FirstPersonGameMode.BP_FirstPersonGameMode_C|GetInventory _asbp_first_person_game_mode) "Power Cell" (Variables|/Game/Blueprint/GameInstace/BP_MyGameInstance.BP_MyGameInstance_C|GetPlayerInventory _asbp_my_game_instance))))
          (bind _returnvalue (UserInterface|CreateWidget "/Game/UI/WBP_Win.WBP_Win_C"))
          (Variables|/Game/UI/WBP_Win.WBP_Win_C|SetLinkedList _returnvalue (Variables|Default|GetLinkedList1))
          (UserInterface|Viewport|AddtoViewport _returnvalue 0)
          (else
            (bind _returnvalue_2 (UserInterface|CreateWidget "/Game/UI/W_Text.W_Text_C" :!label _label))
            (Variables|Default|SetWidgetReference _returnvalue_2)
            (Variables|/Script/UMG.TextBlock|SetText (Variables|/Game/UI/W_Text.W_Text_C|GetTextBlock_0 _returnvalue_2) "You need 4 Power Cells to open this door")
            (UserInterface|Viewport|AddtoViewport _returnvalue_2 0)
            (Utilities|FlowControl|Delay 2.0)
            (Widget|RemovefromParent _returnvalue_2)
            (Variables|Default|SetWidgetReference 0)))
        (else
          (goto _label))))))

(fn ConstructionScript
  (|CallParentFunction))