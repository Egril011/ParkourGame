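; BP_PowerCell_LinkedList is a hand-built singly linked list of power cell records, each holding a name, remaining time and visited flag.
; Append constructs a BPO_PowerCellNode object and initializes it through its Node function.
; The new node becomes Head when the list is empty; otherwise a loop follows NextNode from Head and links it at the tail.
; No tail reference is used, so each append walks the whole list.
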(fn ConstructionScript)

(fn Append
  (params (PowerCellName :type String) (RemaingTime :type Float%20%28double-precision%29) (Visited :type Boolean))
  (LocalVariables|SetPowerCell_Name PowerCellName)
  (LocalVariables|SetRemainggTime RemaingTime)
  (LocalVariables|SetAlreadyVisited Visited)
  (Utilities|IsValid (Variables|Components|GetHead)
    (:Is%20Valid
      (LocalVariables|SetCurrent (Variables|Components|GetHead))
      (while (Utilities|IsValid (Variables|/Game/Blueprint/LinkedList/BPO_PowerCellNode.BPO_PowerCellNode_C|GetNextNode (LocalVariables|GetCurrent)))
        (LocalVariables|SetCurrent (Variables|/Game/Blueprint/LinkedList/BPO_PowerCellNode.BPO_PowerCellNode_C|GetNextNode (LocalVariables|GetCurrent))))
      (bind _returnvalue (Game|ConstructObjectfromClass "/Game/Blueprint/LinkedList/BPO_PowerCellNode.BPO_PowerCellNode_C"))
      (bind _ref (Default|Node _returnvalue (LocalVariables|GetPowerCell_Name) (LocalVariables|GetRemainggTime) (LocalVariables|GetAlreadyVisited)))
      (Variables|/Game/Blueprint/LinkedList/BPO_PowerCellNode.BPO_PowerCellNode_C|SetNextNode (LocalVariables|GetCurrent) _ref)
      (return))
    (:Is%20Not%20Valid
      (bind _returnvalue_2 (Game|ConstructObjectfromClass "/Game/Blueprint/LinkedList/BPO_PowerCellNode.BPO_PowerCellNode_C"))
      (bind _ref_2 (Default|Node _returnvalue_2 (LocalVariables|GetPowerCell_Name) (LocalVariables|GetRemainggTime) (LocalVariables|GetAlreadyVisited)))
      (Variables|Components|SetHead _ref_2)
      (return))))