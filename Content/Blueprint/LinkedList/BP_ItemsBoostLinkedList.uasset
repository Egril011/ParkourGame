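; BP_ItemsBoostLinkedList is a singly linked list that stores item boosts, each with a boost value and a remaining time.
; Append builds a node object, initialized through its Node function, and makes it the Head when none is valid.
; Otherwise it walks the NextNode references from Head and attaches the new BPO_BoostNode at the tail.
; The file only adds entries, with no removal or countdown logic.
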(fn ConstructionScript)

(fn Append
  (params (BoostValue :type Float%20%28double-precision%29) (RemaingTime :type Float%20%28double-precision%29))
  (LocalVariables|SetBooostValue BoostValue)
  (LocalVariables|SetRemainggTime RemaingTime)
  (Utilities|IsValid (Variables|Components|GetHead)
    (:Is%20Valid
      (LocalVariables|SetCurrent (Variables|Components|GetHead))
      (while (Utilities|IsValid (Variables|/Game/Blueprint/LinkedList/BPO_BoostNode.BPO_BoostNode_C|GetNextNode (LocalVariables|GetCurrent)))
        (LocalVariables|SetCurrent (Variables|/Game/Blueprint/LinkedList/BPO_BoostNode.BPO_BoostNode_C|GetNextNode (LocalVariables|GetCurrent))))
      (bind _returnvalue (Game|ConstructObjectfromClass "/Game/Blueprint/LinkedList/BPO_BoostNode.BPO_BoostNode_C"))
      (bind _ref (Default|Node _returnvalue (LocalVariables|GetBooostValue) (LocalVariables|GetRemainggTime)))
      (Variables|/Game/Blueprint/LinkedList/BPO_BoostNode.BPO_BoostNode_C|SetNextNode (LocalVariables|GetCurrent) _ref)
      (return))
    (:Is%20Not%20Valid
      (bind _returnvalue_2 (Game|ConstructObjectfromClass "/Game/Blueprint/LinkedList/BPO_BoostNode.BPO_BoostNode_C"))
      (bind _ref_2 (Default|Node _returnvalue_2 (LocalVariables|GetBooostValue) (LocalVariables|GetRemainggTime)))
      (Variables|Components|SetHead _ref_2)
      (return))))