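; Power cell combo tracker that rewards quick successive entries in a linked list with combo points stored in BP_MyGameInstance.
; StartTimerCombo restarts a looping timer that runs Combo, which walks the list while the combo window is open.
; Each unvisited node scores tiered points by its TimeRemaining gap from the previous node.
; WBP_Combo appears once two nodes exist; when the window expires, it is removed and PlayerCombo resets.
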(event EventBeginPlay)

(event Collision|EventActorBeginOverlap
  (params (OtherActor :type Actor%20Object%20Reference)))

(event EventTick
  (params (DeltaSeconds :type Float%20%28single-precision%29)))

(fn ConstructionScript)

(fn Combo
  (bind _output_get (Variables|Default|SetComboTimer (+ (Variables|Default|GetTime) (Variables|Default|GetComboTimer))))
  (if (< _output_get 25.0)
    (Variables|Default|SetCurrent (Variables|/Game/Blueprint/LinkedList/BP_PowerCell_LinkedList.BP_PowerCell_LinkedList_C|GetHead (Variables|Default|GetLinkedList)))
    (Variables|Default|SetLastCurrent (Variables|Default|GetCurrent))
    (while (Utilities|IsValid (Variables|Default|GetCurrent))
      (if (== (Variables|Default|GetCurrent) (Variables|/Game/Blueprint/LinkedList/BP_PowerCell_LinkedList.BP_PowerCell_LinkedList_C|GetHead (Variables|Default|GetLinkedList)))
        _
        (else
          (CallFunction|SetPlayerComboPoints (Variables|/Game/Blueprint/LinkedList/BPO_PowerCellNode.BPO_PowerCellNode_C|GetTimeRemaining (Variables|Default|GetCurrent)) (Variables|/Game/Blueprint/LinkedList/BPO_PowerCellNode.BPO_PowerCellNode_C|GetTimeRemaining (Variables|Default|GetLastCurrent)))))
      (Variables|Default|SetLastCurrent (Variables|Default|GetCurrent))
      (Variables|Default|SetCurrent (Variables|/Game/Blueprint/LinkedList/BPO_PowerCellNode.BPO_PowerCellNode_C|GetNextNode (Variables|Default|GetCurrent))))
    (if (Utilities|IsValid (Variables|/Game/Blueprint/LinkedList/BPO_PowerCellNode.BPO_PowerCellNode_C|GetNextNode (Variables|/Game/Blueprint/LinkedList/BP_PowerCell_LinkedList.BP_PowerCell_LinkedList_C|GetHead (Variables|Default|GetLinkedList))))
      (Utilities|IsValid (Variables|Default|GetWidgetRef)
        (:Is%20Not%20Valid
          (bind _returnvalue (UserInterface|CreateWidget "/Game/UI/WBP_Combo.WBP_Combo_C"))
          (bind _output_get_2 (Variables|Default|SetWidgetRef _returnvalue))
          (UserInterface|Viewport|AddtoViewport _output_get_2 0))))
    (else
      (Utilities|IsValid (Variables|Default|GetWidgetRef)
        (:Is%20Valid
          (Widget|RemovefromParent (Variables|Default|GetWidgetRef))
          (Variables|Default|SetWidgetRef 0)
          (bind _asbp_my_game_instance (Utilities|Casting|CastToBP_MyGameInstance (Game|GetGameInstance)))
          (Variables|/Game/Blueprint/GameInstace/BP_MyGameInstance.BP_MyGameInstance_C|SetPlayerCombo _asbp_my_game_instance 0.0))))))

(fn StartTimerCombo
  (Variables|Default|SetComboTimer 0.0)
  (Utilities|Time|SetTimerbyFunctionName 0 "Combo" (Variables|Default|GetTime) true))

(fn SetPlayerComboPoints
  (params (FirstTime :type Float%20%28double-precision%29) (SecondTime :type Float%20%28double-precision%29))
  (bind _returnvalue (- SecondTime FirstTime))
  (if (Variables|/Game/Blueprint/LinkedList/BPO_PowerCellNode.BPO_PowerCellNode_C|GetVisited (Variables|Default|GetCurrent))
    (return)
    (elif (< _returnvalue 15.0)
      (bind _asbp_my_game_instance (Utilities|Casting|CastToBP_MyGameInstance (Game|GetGameInstance)))
      (Variables|/Game/Blueprint/GameInstace/BP_MyGameInstance.BP_MyGameInstance_C|SetPlayerCombo _asbp_my_game_instance (+ (Variables|/Game/Blueprint/GameInstace/BP_MyGameInstance.BP_MyGameInstance_C|GetPlayerCombo _asbp_my_game_instance) 2e+01))
      (Variables|/Game/Blueprint/LinkedList/BPO_PowerCellNode.BPO_PowerCellNode_C|SetVisited (Variables|Default|GetCurrent) true)
      (return)
      (elif (< _returnvalue 2e+01)
        (bind _asbp_my_game_instance_2 (Utilities|Casting|CastToBP_MyGameInstance (Game|GetGameInstance)))
        (Variables|/Game/Blueprint/GameInstace/BP_MyGameInstance.BP_MyGameInstance_C|SetPlayerCombo _asbp_my_game_instance_2 (+ (Variables|/Game/Blueprint/GameInstace/BP_MyGameInstance.BP_MyGameInstance_C|GetPlayerCombo _asbp_my_game_instance_2) 1e+01))
        (Variables|/Game/Blueprint/LinkedList/BPO_PowerCellNode.BPO_PowerCellNode_C|SetVisited (Variables|Default|GetCurrent) true)
        (return)
        (elif (< _returnvalue 25.0)
          (bind _asbp_my_game_instance_3 (Utilities|Casting|CastToBP_MyGameInstance (Game|GetGameInstance)))
          (Variables|/Game/Blueprint/GameInstace/BP_MyGameInstance.BP_MyGameInstance_C|SetPlayerCombo _asbp_my_game_instance_3 (+ (Variables|/Game/Blueprint/GameInstace/BP_MyGameInstance.BP_MyGameInstance_C|GetPlayerCombo _asbp_my_game_instance_3) 5.0))
          (Variables|/Game/Blueprint/LinkedList/BPO_PowerCellNode.BPO_PowerCellNode_C|SetVisited (Variables|Default|GetCurrent) true)
          (return)
          (else
            (Variables|/Game/Blueprint/LinkedList/BPO_PowerCellNode.BPO_PowerCellNode_C|SetVisited (Variables|Default|GetCurrent) true)
            (Variables|Default|SetCurrent (Variables|/Game/Blueprint/LinkedList/BPO_PowerCellNode.BPO_PowerCellNode_C|GetNextNode (Variables|Default|GetCurrent)))))))))